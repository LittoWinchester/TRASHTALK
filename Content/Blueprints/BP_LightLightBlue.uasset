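; Quest light actor that marks an interaction spot where the player completes an item quest.
; Tick polls BP_character's Light flag to toggle the light and box overlaps, and overlap drives a press-E prompt.
; Interacting while touching with a quest item adds progress, kills the light, plays sounds including one from DT_ItemsTrash, and shows a completion widget.
; A DoOnce limits this to once until it is reset by interacting without an item.
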(event `ShowPressE`
  ;[1 1 1] Function Show And Hide
  (`Widget.SetVisibility` (`self.E`) "Visible"))

(event `self.ReceiveBeginPlay`
  (`LightComponent.SetIntensity` (`self.LightComponent`) 0.0)
  (bind _returnvalue (`|CreateWidget` "/Game/UI/UI_PressE.UI_PressE_C"))
  (set `self.E` _returnvalue)
  (`UserWidget.AddToViewport` (`self.E`) 0)
  (`Widget.SetVisibility` (`self.E`) "Collapsed"))

(event `HidePressE`
  ;[1 1 1] Function Show And Hide
  (`Widget.SetVisibility` (`self.E`) "Hidden"))

(event `self.ReceiveTick`
  (params (DeltaSeconds :type "Float (single-precision)"))
  (`self.Quest creating`)
  (`self.QuestCompleted`))

(event `Quest creating`
  (bind _box (`self.Box`))
  ;[1 1 1] Questing
  (bind _asbp_character (cast `/Game/Blueprints/BP_character` (`GameplayStatics.GetPlayerCharacter` 0)))
  (if (`/Game/Blueprints/BP_character.light` _asbp_character)
    (`LightComponent.SetIntensity` (`self.LightComponent`) 25.0)
    (set `PrimitiveComponent.bGenerateOverlapEvents` true _box)
    (else
      (`LightComponent.SetIntensity` (`self.LightComponent`) 0.0)
      (set `PrimitiveComponent.bGenerateOverlapEvents` false _box))))

(event `self.ReceiveActorBeginOverlap`
  (params (OtherActor :type "Actor Object Reference"))
  ;[1 1 1] Overlap
  (if (== OtherActor (`GameplayStatics.GetPlayerCharacter` 0))
    (`UserWidget.AddToViewport` (`self.E`) 0)
    (`self.ShowPressE`)
    (set `self.touching` true)
    (bind _asbp_character (cast `/Game/Blueprints/BP_character` (`GameplayStatics.GetPlayerCharacter` 0)))
    (set `/Game/Blueprints/BP_character.InteractionON` false _asbp_character)))

(event `self.Box.OnComponentEndOverlap`
  (params (OverlappedComponent :type "PrimitiveComponent Object Reference") (OtherActor :type "Actor Object Reference") (OtherComp :type "PrimitiveComponent Object Reference") (OtherBodyIndex :type Integer))
  ;[1 1 1] Overlap
  (if (== (`GameplayStatics.GetPlayerCharacter` 0) OtherActor)
    (`Widget.RemoveFromParent` (`self.E`))
    (`self.HidePressE`)
    (set `self.touching` false)
    (bind _asbp_character (cast `/Game/Blueprints/BP_character` (`GameplayStatics.GetPlayerCharacter` 0)))
    (set `/Game/Blueprints/BP_character.InteractionON` false _asbp_character)))

(event `TilinFn`
  ;[1 1 1] Tilin
  (`GameplayStatics.PlaySound2D` "/Game/Sound/tilin_2.tilin_2" 1.0 1.0 0.0 null null)
  (`KismetSystemLibrary.Delay` 0.5)
  (bind _returnvalue (`|CreateWidget` "/Game/UI/UI_QuestCompleted.UI_QuestCompleted_C"))
  (`UserWidget.AddToViewport` _returnvalue 0)
  (bind _returnvalue_2 (`GameplayStatics.GetActorOfClass` "/Game/Blueprints/BP_character.BP_character_C"))
  (bind _returnvalue_3 (`|GetDataTableRow` "/Game/Data/DT_ItemsTrash.DT_ItemsTrash" (`KismetStringLibrary.Conv_StringToName` (`/Game/Blueprints/BP_character.VarSoundQuest` _returnvalue_2)))
    (:`then`
      (`GameplayStatics.PlaySound2D` (`.SoundQuestComplete_34_F86E09D846A96B3D890FCDBE36F7294A` (break `/Game/Data/DT_DataStructure` _returnvalue_3)) 1.0 1.0 0.0 null null))))

(event `QuestCompleted`
  ;[1 1 1] Activate Quest Light
  (if (`self.Touching`)
    (bind _asbp_character (cast `/Game/Blueprints/BP_character` (`GameplayStatics.GetPlayerCharacter` 0)))
    (if (`/Game/Blueprints/BP_character.InteractionON` _asbp_character)
      (set `/Game/Blueprints/BP_character.CameraOn` true _asbp_character)
      (`self.HidePressE`)
      (if (`KismetStringLibrary.NotEqual_StrStr` (`/Game/Blueprints/BP_character.ItemQuest` _asbp_character))
        (`/Engine/EditorBlueprintResources/StandardMacros.DoOnce` false :!label _label
          (:`Completed`
            (set `/Game/Blueprints/BP_character.ProgresBar` (+ (`/Game/Blueprints/BP_character.ProgresBar` _asbp_character) 25.0) _asbp_character)
            (`LightComponent.SetIntensity` (`self.LightComponent`) 0.0)
            (`self.TilinFn`)))
        (else
          (goto _label :!via `Reset`)))
      (else
        (set `/Game/Blueprints/BP_character.CameraOn` true _asbp_character)
        (`self.ShowPressE`)))))

(fn `UserConstructionScript`)